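; PC_player is a player controller that turns Enhanced Input actions into movement and jumping for BP_Character.
; On BeginPlay it caches the player 0 pawn as BP_Character and adds IMC_Mapping, printing a message if the cast fails.
; IA_move drives movement along the character's forward (X) and right (Y) vectors.
; IA_jump starts and stops jumping, printing a debug string once held for two seconds or longer.
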(event Input|EnhancedActionEvents|EnhancedInputActionIA_jump
  (params (ActionValue :type Boolean) (ElapsedSeconds :type Float%20%28double-precision%29) (TriggeredSeconds :type Float%20%28double-precision%29) (InputAction :type Input%20Action%20Object%20Reference :default "/Game/Input/IA_jump.IA_jump"))
  (bind _as_bp_character (Variables|Default|GetAs%20BP%20Character))
  (:Triggered
    (if (> 2.0 TriggeredSeconds)
      _
      (else
        (Development|PrintString "MAthis")))
    (Character|Jump _as_bp_character))
  (:Completed
    (Character|StopJumping _as_bp_character)))

(event Input|EnhancedActionEvents|EnhancedInputActionIA_move
  (params (ActionValue :type Vector%202D%20Structure) (ElapsedSeconds :type Float%20%28double-precision%29) (TriggeredSeconds :type Float%20%28double-precision%29) (InputAction :type Input%20Action%20Object%20Reference :default "/Game/Input/IA_move.IA_move"))
  (bind (_x _y) (Math|Vector2D|BreakVector2D ActionValue))
  (bind _as_bp_character (Variables|Default|GetAs%20BP%20Character))
  (:Triggered
    (Pawn|Input|AddMovementInput _as_bp_character (Transformation|GetActorForwardVector _as_bp_character) _x false)
    (Pawn|Input|AddMovementInput _as_bp_character (Transformation|GetActorRightVector _as_bp_character) _y false)))

(event EventBeginPlay
  (bind _asbp_character (Utilities|Casting|CastToBP_Character (Game|Player|GetPlayerPawn 0))
    (:then
      (Variables|Default|SetAs%20BP%20Character _asbp_character)
      (Input|AddMappingContext (PlayerController|LocalPlayerSubsystems|GetEnhancedInputLocalPlayerSubsystem self) "/Game/Input/IMC_Mapping.IMC_Mapping" 0 "(bIgnoreAllPressedKeysUntilRelease=True,bForceImmediately=False,bNotifyUserSettings=False)"))
    (:CastFailed
      (Development|PrintString "Character cast failed"))))

(fn ConstructionScript)