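; Player controller that turns Enhanced Input actions into actions on the possessed BP_Character.
; BeginPlay caches the character and adds the mapping context; input events then drive look, movement, jumping and grenade-type cycling.
; Crouch is simulated by lowering the spring arm and halving movement input.
; The save action copies grenade count and new-weapon data from GI_MainInstance into an SG_gameSave slot.
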(event Input|EnhancedActionEvents|EnhancedInputActionIA_jump
  (params (ActionValue :type Boolean) (ElapsedSeconds :type Float%20%28double-precision%29) (TriggeredSeconds :type Float%20%28double-precision%29) (InputAction :type Input%20Action%20Object%20Reference :default "/Game/Input/IA_jump.IA_jump"))
  (bind _as_bp_character (Variables|Default|GetAs%20BP%20Character))
  ;[1 1 1] Jumping
  (:Triggered
    (if (> (Variables|Default|GetTimeToTrigger) TriggeredSeconds)
      _
      (else
        (Development|PrintString "MAthis")))
    (Character|Jump _as_bp_character))
  (:Completed
    (Character|StopJumping _as_bp_character)))

(event Input|EnhancedActionEvents|EnhancedInputActionIA_move
  (params (ActionValue :type Vector%202D%20Structure) (ElapsedSeconds :type Float%20%28double-precision%29) (TriggeredSeconds :type Float%20%28double-precision%29) (InputAction :type Input%20Action%20Object%20Reference :default "/Game/Input/IA_move.IA_move"))
  (bind (_x _y) (Math|Vector2D|BreakVector2D ActionValue))
  (bind _as_bp_character (Variables|Default|GetAs%20BP%20Character))
  ;[1 1 1] Movement
  (if (Variables|Default|GetCrouch?)
    (Variables|Default|SetSpeedMultiplicater 0.5)
    (else
      (bind _output_get (Variables|Default|SetSpeedMultiplicater 1.0))))
  (Pawn|Input|AddMovementInput _as_bp_character (Transformation|GetActorForwardVector _as_bp_character) (* _x _output_get) false)
  (Pawn|Input|AddMovementInput _as_bp_character (Transformation|GetActorRightVector _as_bp_character) (* _y _output_get) false))

(event Input|EnhancedActionEvents|EnhancedInputActionIA_CameraLook
  (params (ActionValue :type Vector%202D%20Structure) (ElapsedSeconds :type Float%20%28double-precision%29) (TriggeredSeconds :type Float%20%28double-precision%29) (InputAction :type Input%20Action%20Object%20Reference :default "/Game/Input/IA_CameraLook.IA_CameraLook"))
  (bind _as_bp_character (Variables|Default|GetAs%20BP%20Character))
  ;[1 1 1] Camera
  (Pawn|Input|AddControllerYawInput _as_bp_character (/ (.x ActionValue) 2.0))
  (Pawn|Input|AddControllerPitchInput _as_bp_character (/ (.y ActionValue) 2.0))
  (Pawn|Input|AddControllerPitchInput _as_bp_character (* (Class|Actor|GetInputAxisKeyValue) -1.0)))

(event Input|EnhancedActionEvents|EnhancedInputActionIA_Save
  (params (ActionValue :type Boolean) (ElapsedSeconds :type Float%20%28double-precision%29) (TriggeredSeconds :type Float%20%28double-precision%29) (InputAction :type Input%20Action%20Object%20Reference :default "/Game/Input/IA_Save.IA_Save"))
  (:Started
    (bind _asgi_main_instance (Utilities|Casting|CastToGI_MainInstance (Game|GetGameInstance)))
    (bind _returnvalue (SaveGame|CreateSaveGameObject "/Game/Manage/SG_gameSave.SG_gameSave_C"))
    (Variables|/Game/Manage/SG_gameSave.SG_gameSave_C|SetGrenadesnb _returnvalue (Variables|/Game/Manage/GI_MainInstance.GI_MainInstance_C|GetGrenadeNb _asgi_main_instance))
    (Variables|/Game/Manage/SG_gameSave.SG_gameSave_C|SetNewWeapon _returnvalue (Variables|/Game/Manage/GI_MainInstance.GI_MainInstance_C|GetNewWeapon _asgi_main_instance))
    (SaveGame|SaveGametoSlot _returnvalue "Save")))

(event Input|EnhancedActionEvents|EnhancedInputActionIA_ChangeNade
  (params (ActionValue :type Float%20%28double-precision%29) (ElapsedSeconds :type Float%20%28double-precision%29) (TriggeredSeconds :type Float%20%28double-precision%29) (InputAction :type Input%20Action%20Object%20Reference :default "/Game/Input/IA_ChangeNade.IA_ChangeNade"))
  (bind _as_bp_character (Variables|Default|GetAs%20BP%20Character))
  ;[1 1 1] Change Bombs
  (:Started
    (Variables|/Game/Character/BP_Character.BP_Character_C|SetGrenadeType _as_bp_character (Math|Float|Truncate (+ ActionValue (Variables|/Game/Character/BP_Character.BP_Character_C|GetGrenadeType _as_bp_character))))
    (if (< (Math|Float|Truncate (+ ActionValue (Variables|/Game/Character/BP_Character.BP_Character_C|GetGrenadeType _as_bp_character))) -1)
      (Variables|/Game/Character/BP_Character.BP_Character_C|SetGrenadeType _as_bp_character 3)
      (elif (> (Math|Float|Truncate (+ ActionValue (Variables|/Game/Character/BP_Character.BP_Character_C|GetGrenadeType _as_bp_character))) 4)
        (Variables|/Game/Character/BP_Character.BP_Character_C|SetGrenadeType _as_bp_character 0)))
    (Development|PrintString (Utilities|String|ToString(Integer) (Variables|/Game/Character/BP_Character.BP_Character_C|GetGrenadeType _as_bp_character)))))

(event Input|EnhancedActionEvents|EnhancedInputActionIA_Crouch
  (params (ActionValue :type Boolean) (ElapsedSeconds :type Float%20%28double-precision%29) (TriggeredSeconds :type Float%20%28double-precision%29) (InputAction :type Input%20Action%20Object%20Reference :default "/Game/Input/IA_Crouch.IA_Crouch"))
  (bind _as_bp_character (Variables|Default|GetAs%20BP%20Character))
  (bind _springarm (Variables|/Game/Character/BP_Character.BP_Character_C|GetSpringArm _as_bp_character))
  (bind _returnvalue (Transformation|GetWorldLocation _springarm))
  ;[1 1 1] Crouch
  (:Started
    (bind _output_get (Variables|Default|SetBaseCamPos _returnvalue))
    (Transformation|SetWorldLocation _springarm (Math|Vector|MakeVector (.x _output_get) (.y _output_get) (- (.z _output_get) 2e+01)) false false)
    (Variables|Default|SetCrouch? true))
  (:Completed
    (bind _output_get_2 (Variables|Default|SetBaseCamPos _returnvalue))
    (Transformation|SetWorldLocation _springarm (Math|Vector|MakeVector (.x _output_get_2) (.y _output_get_2) (- (.z _output_get_2) -2e+01)) false false)
    (Variables|Default|SetCrouch? false)))

(event EventBeginPlay
  ;[1 1 1] Initiate cast and input
  (bind _asbp_character (Utilities|Casting|CastToBP_Character (Game|Player|GetPlayerPawn 0))
    (:then
      (Variables|Default|SetAs%20BP%20Character _asbp_character)
      (Input|AddMappingContext (PlayerController|LocalPlayerSubsystems|GetEnhancedInputLocalPlayerSubsystem self) "/Game/Input/IMC_Mapping.IMC_Mapping" 0 "(bIgnoreAllPressedKeysUntilRelease=True,bForceImmediately=False,bNotifyUserSettings=False)"))
    (:CastFailed
      (Development|PrintString "Character cast failed"))))

(fn ConstructionScript)