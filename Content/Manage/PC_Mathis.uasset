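; Player controller that adds the Enhanced Input mapping on BeginPlay and drives the possessed BP_Character.
; It handles look, movement, jump and a hold crouch that lowers the spring arm and halves movement input.
; Input also toggles two weapons and cycles grenade type on the character.
; Shooting line-traces from the camera, repeating at short range or single-shot at long range via a delayed DoOnce reset, and only prints debug text.
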(event Input|EnhancedActionEvents|EnhancedInputActionIA_jump
  (params (ActionValue :type Boolean) (ElapsedSeconds :type Float%20%28double-precision%29) (TriggeredSeconds :type Float%20%28double-precision%29) (InputAction :type Input%20Action%20Object%20Reference :default "/Game/Input/IA_jump.IA_jump"))
  (bind _as_bp_character (Variables|Default|GetAs%20BP%20Character))
  ;[1 1 1] Jumping
  (:Triggered
    (if (> (Variables|Default|GetTimeToTrigger) TriggeredSeconds)
      _
      (else
        (Development|PrintString "MAthis")))
    (Character|Jump _as_bp_character))
  (:Completed
    (Character|StopJumping _as_bp_character)))

(event Input|EnhancedActionEvents|EnhancedInputActionIA_move
  (params (ActionValue :type Vector%202D%20Structure) (ElapsedSeconds :type Float%20%28double-precision%29) (TriggeredSeconds :type Float%20%28double-precision%29) (InputAction :type Input%20Action%20Object%20Reference :default "/Game/Input/IA_move.IA_move"))
  (bind (_x _y) (Math|Vector2D|BreakVector2D ActionValue))
  (bind _as_bp_character (Variables|Default|GetAs%20BP%20Character))
  ;[1 1 1] Movement
  (if (Variables|Default|GetCrouch?)
    (Variables|Default|SetSpeedMultiplicater 0.5)
    (else
      (bind _output_get (Variables|Default|SetSpeedMultiplicater 1.0))))
  (Pawn|Input|AddMovementInput _as_bp_character (Transformation|GetActorForwardVector _as_bp_character) (* _x _output_get) false)
  (Pawn|Input|AddMovementInput _as_bp_character (Transformation|GetActorRightVector _as_bp_character) (* _y _output_get) false))

(event Input|EnhancedActionEvents|EnhancedInputActionIA_Shoot
  (params (ActionValue :type Boolean) (ElapsedSeconds :type Float%20%28double-precision%29) (TriggeredSeconds :type Float%20%28double-precision%29) (InputAction :type Input%20Action%20Object%20Reference :default "/Game/Input/IA_Shoot.IA_Shoot"))
  (bind _as_bp_character (Variables|Default|GetAs%20BP%20Character))
  (bind _as_bp_character_2 (Variables|Default|GetAs%20BP%20Character))
  (bind _array (Utilities|Array|MakeArray _as_bp_character_2))
  (bind _camera (Variables|/Game/Character/BP_Character.BP_Character_C|GetCamera _as_bp_character))
  (bind _returnvalue (Transformation|GetWorldLocation _camera))
  (bind _returnvalue_2 (Transformation|GetWorldRotation _camera))
  (bind _returnvalue_3 (Math|Vector|GetForwardVector _returnvalue_2))
  ;[1 1 1] Shoot
  (:Triggered
    (if (Variables|/Game/Character/BP_Character.BP_Character_C|GetFirstWeapon? _as_bp_character)
      (Utilities|FlowControl|Delay 0.1)
      (bind _returnvalue_4 (Collision|LineTraceByChannel _returnvalue (+ _returnvalue (* _returnvalue_3 1e+03)) "TraceTypeQuery1" false _array "None"))
      (Development|PrintString "Piou")
      (if _returnvalue_4
        (Development|PrintString "Touched!" :!label _label))
      (else
        (Utilities|FlowControl|DoOnce false :!label _label_2
          (:Completed
            (bind _returnvalue_5 (Collision|LineTraceByChannel _returnvalue (+ _returnvalue (* _returnvalue_3 1e+04)) "TraceTypeQuery1" false _array "None"))
            (Development|PrintString "PIOUUUU!!!")
            (if _returnvalue_5
              (goto _label)))))))
  (:Completed
    (Utilities|FlowControl|Delay 1.0)
    (goto _label_2 Reset)))

(event Input|EnhancedActionEvents|EnhancedInputActionIA_CameraLook
  (params (ActionValue :type Vector%202D%20Structure) (ElapsedSeconds :type Float%20%28double-precision%29) (TriggeredSeconds :type Float%20%28double-precision%29) (InputAction :type Input%20Action%20Object%20Reference :default "/Game/Input/IA_CameraLook.IA_CameraLook"))
  (bind _as_bp_character (Variables|Default|GetAs%20BP%20Character))
  ;[1 1 1] Camera
  (Pawn|Input|AddControllerYawInput _as_bp_character (/ (.x ActionValue) 2.0))
  (Pawn|Input|AddControllerPitchInput _as_bp_character (/ (.y ActionValue) 2.0))
  (Pawn|Input|AddControllerPitchInput _as_bp_character (* (Class|Actor|GetInputAxisKeyValue) -1.0)))

(event Input|EnhancedActionEvents|EnhancedInputActionIA_ChangeGun
  (params (ActionValue :type Boolean) (ElapsedSeconds :type Float%20%28double-precision%29) (TriggeredSeconds :type Float%20%28double-precision%29) (InputAction :type Input%20Action%20Object%20Reference :default "/Game/Input/IA_ChangeGun.IA_ChangeGun"))
  (bind _as_bp_character (Variables|Default|GetAs%20BP%20Character))
  ;[1 1 1] Change WP
  (if ActionValue
    (if (Variables|/Game/Character/BP_Character.BP_Character_C|GetFirstWeapon? _as_bp_character)
      (Variables|/Game/Character/BP_Character.BP_Character_C|SetFirstWeapon? _as_bp_character false)
      (else
        (Variables|/Game/Character/BP_Character.BP_Character_C|SetFirstWeapon? _as_bp_character true)))))

(event Input|EnhancedActionEvents|EnhancedInputActionIA_ChangeNade
  (params (ActionValue :type Float%20%28double-precision%29) (ElapsedSeconds :type Float%20%28double-precision%29) (TriggeredSeconds :type Float%20%28double-precision%29) (InputAction :type Input%20Action%20Object%20Reference :default "/Game/Input/IA_ChangeNade.IA_ChangeNade"))
  (bind _as_bp_character (Variables|Default|GetAs%20BP%20Character))
  ;[1 1 1] Change Bombs
  (:Started
    (Variables|/Game/Character/BP_Character.BP_Character_C|SetGrenadeType _as_bp_character (Math|Float|Truncate (+ ActionValue (Variables|/Game/Character/BP_Character.BP_Character_C|GetGrenadeType _as_bp_character))))
    (if (< (Math|Float|Truncate (+ ActionValue (Variables|/Game/Character/BP_Character.BP_Character_C|GetGrenadeType _as_bp_character))) -1)
      (Variables|/Game/Character/BP_Character.BP_Character_C|SetGrenadeType _as_bp_character 3)
      (elif (> (Math|Float|Truncate (+ ActionValue (Variables|/Game/Character/BP_Character.BP_Character_C|GetGrenadeType _as_bp_character))) 4)
        (Variables|/Game/Character/BP_Character.BP_Character_C|SetGrenadeType _as_bp_character 0)))
    (Development|PrintString (Utilities|String|ToString(Integer) (Variables|/Game/Character/BP_Character.BP_Character_C|GetGrenadeType _as_bp_character)))))

(event Input|EnhancedActionEvents|EnhancedInputActionIA_Crouch
  (params (ActionValue :type Boolean) (ElapsedSeconds :type Float%20%28double-precision%29) (TriggeredSeconds :type Float%20%28double-precision%29) (InputAction :type Input%20Action%20Object%20Reference :default "/Game/Input/IA_Crouch.IA_Crouch"))
  (bind _as_bp_character (Variables|Default|GetAs%20BP%20Character))
  (bind _springarm (Variables|/Game/Character/BP_Character.BP_Character_C|GetSpringArm _as_bp_character))
  (bind _returnvalue (Transformation|GetWorldLocation _springarm))
  ;[1 1 1] Crouch
  (:Started
    (bind _output_get (Variables|Default|SetBaseCamPos _returnvalue))
    (Transformation|SetWorldLocation _springarm (Math|Vector|MakeVector (.x _output_get) (.y _output_get) (- (.z _output_get) 2e+01)) false false)
    (Variables|Default|SetCrouch? true))
  (:Completed
    (bind _output_get_2 (Variables|Default|SetBaseCamPos _returnvalue))
    (Transformation|SetWorldLocation _springarm (Math|Vector|MakeVector (.x _output_get_2) (.y _output_get_2) (- (.z _output_get_2) -2e+01)) false false)
    (Variables|Default|SetCrouch? false)))

(event EventBeginPlay
  ;[1 1 1] Initiate cast and input
  (bind _asbp_character (Utilities|Casting|CastToBP_Character (Game|Player|GetPlayerPawn 0))
    (:then
      (Variables|Default|SetAs%20BP%20Character _asbp_character)
      (Input|AddMappingContext (PlayerController|LocalPlayerSubsystems|GetEnhancedInputLocalPlayerSubsystem self) "/Game/Input/IMC_Mapping.IMC_Mapping" 0 "(bIgnoreAllPressedKeysUntilRelease=True,bForceImmediately=False,bNotifyUserSettings=False)"))
    (:CastFailed
      (Development|PrintString "Character cast failed"))))

(fn ConstructionScript)