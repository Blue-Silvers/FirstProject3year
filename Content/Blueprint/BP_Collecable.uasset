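; BP_Collecable is a pickup actor that gives the player either grenades or healing, chosen by its Grenade flag.
; In grenade mode, BeginPlay sets the child actor's class from GrenadeBPClass by GrenadeType.
; Sphere overlap with a player-tagged BP_Character adds grenades and destroys the pickup only while that type's count is under the cap.
; Otherwise it calls AddHeal with Value and does not destroy itself.
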(event OnComponentBeginOverlap(Sphere1)
  (params (OverlappedComponent :type Primitive%20Component%20Object%20Reference) (OtherActor :type Actor%20Object%20Reference) (OtherComp :type Primitive%20Component%20Object%20Reference) (OtherBodyIndex :type Integer) (bFromSweep :type Boolean) (SweepResult :type Hit%20Result%20Structure%20%28by%20ref%29))
  (if (Actor|ActorHasTag OtherActor "player")
    (bind _asbp_character (Utilities|Casting|CastToBP_Character OtherActor))
    (if (Variables|Default|GetGrenade?)
      (if (<= (Utilities|Array|Get(acopy) (Variables|/Game/Character/BP_Character.BP_Character_C|GetGrenadeNb _asbp_character) (Variables|Default|GetGrenadeType)) 4)
        (Actor|DestroyActor)
        (Default|AddGrenade _asbp_character (Variables|Default|GetValue) (Variables|Default|GetGrenadeType)))
      (else
        (Default|AddHeal _asbp_character (Variables|Default|GetValue))))))

(event EventBeginPlay
  (if (Variables|Default|GetGrenade?)
    (ChildActorComponent|SetChildActorClass (Variables|Default|GetChildActor) (Utilities|Array|Get(acopy) (Variables|Default|GetGrenade_BP_Class) (Variables|Default|GetGrenadeType)))))

(fn ConstructionScript)