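; Grappling hook actor that pulls the player toward a surface while IA_Shoot is held.
; On press, a Visibility line trace along the pawn root's forward vector sets the grab point, switches movement to Flying and shows a cable.
; Tick pins the cable end to that point and adds force toward it; the sideways term is multiplied by zero.
; Release restores Falling and hides the cable; the input also triggers a firing sound call.
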(event Input|EnhancedActionEvents|EnhancedInputActionIA_Shoot
  (params (ActionValue :type Boolean) (ElapsedSeconds :type Float%20%28double-precision%29) (TriggeredSeconds :type Float%20%28double-precision%29) (InputAction :type Input%20Action%20Object%20Reference :default "/Game/Input/IA_Shoot.IA_Shoot"))
  (bind _returnvalue (Game|Player|GetPlayerPawn 0))
  (bind _rootcomponent (Variables|/Script/Engine.Actor|GetRootComponent _returnvalue))
  (bind _returnvalue_2 (Transformation|GetWorldLocation _rootcomponent))
  ;[0 0.4 0.4] Grappling System
  (:Started
    (bind (_outhit _returnvalue_3) (Collision|LineTraceByChannel _returnvalue_2 (+ _returnvalue_2 (* (Math|Vector|GetForwardVector (Transformation|GetWorldRotation _rootcomponent)) 1.5e+03)) "TraceTypeQuery1" false 0 "None"))
    (if _returnvalue_3
      (Variables|Default|SetGrabPoint (.ImpactPoint (Collision|BreakHitResult _outhit)))
      (Variables|Default|SetIsGrappling true)
      (Pawn|Components|CharacterMovement|SetMovementMode (Variables|/Script/Engine.Character|GetCharacterMovement (Game|GetPlayerCharacter 0)) "MOVE_Flying" 0)
      (Rendering|SetVisibility (Variables|Default|GetCable) true false)))
  (:Completed
    (Variables|Default|SetIsGrappling false)
    (Pawn|Components|CharacterMovement|SetMovementMode (Variables|/Script/Engine.Character|GetCharacterMovement (Game|GetPlayerCharacter 0)) "MOVE_Falling" 0)
    (Rendering|SetVisibility (Variables|Default|GetCable) false false)))

(event Input|EnhancedActionEvents|EnhancedInputActionIA_Shoot
  (params (ActionValue :type Boolean) (ElapsedSeconds :type Float%20%28double-precision%29) (TriggeredSeconds :type Float%20%28double-precision%29) (InputAction :type Input%20Action%20Object%20Reference :default "/Game/Input/IA_Shoot.IA_Shoot"))
  ;[0 0.4 0.4] Grappling System
  (Audio|PlaySoundatLocation 0 (Transformation|GetWorldLocation (Variables|/Script/Engine.Actor|GetRootComponent (Game|Player|GetPlayerPawn 0))) "0, 0, 0" 1.0 1.0 0.0 0 0 0 0) ; Play firing sound
)

(event EventBeginPlay
  (|CallParentFunction) ; This node is disabled and will not be called.\nDrag off pins to build functionality.
)

(event Collision|EventActorBeginOverlap
  (params (OtherActor :type Actor%20Object%20Reference))
  (|CallParentFunction OtherActor) ; This node is disabled and will not be called.\nDrag off pins to build functionality.
)

(event EventTick
  (params (DeltaSeconds :type Float%20%28single-precision%29))
  (bind _returnvalue (Game|GetPlayerCharacter 0))
  ;[0 0.4 0.4] Graplling aspect and force
  (if (Variables|Default|GetIsGrappling)
    (Variables|/Script/CableComponent.CableComponent|SetEndLocation (Variables|Default|GetCable) (Math|Transform|InverseTransformLocation (Transformation|GetActorTransform _returnvalue) (Variables|Default|GetGrabPoint)))
    (Physics|AddForce (Variables|/Script/Engine.Character|GetCharacterMovement (Game|GetPlayerCharacter 0)) (* (Math|Vector|Normalize (+ (Math|Vector|GetUnitDirection(Vector) (Transformation|GetActorLocation _returnvalue) (Variables|Default|GetGrabPoint)) (* (* (Transformation|GetActorRightVector _returnvalue) "") 0.7))) 2.5e+05))))

(fn ConstructionScript
  (|CallParentFunction))