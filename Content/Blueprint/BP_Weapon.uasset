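; BP_Weapon is a hitscan weapon Blueprint that fires a line trace and damages the actor it hits.
; Shoot passes a DoOnce into FireWeapon, plays FireSound at the world origin, then immediately calls ResetWeapon to reopen the gate, so no delay limits fire rate.
; FireWeapon traces forward from the Linetrace component over Range against world and pawn objects, ignoring itself and the player, with debug drawing, and applies WeaponDamage.
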(event Custom|Shoot
  (Utilities|FlowControl|DoOnce false
    (:Completed
      (CallFunction|FireWeapon)
      (Audio|PlaySoundatLocation (Variables|Default|GetFireSound) "0, 0, 0" "0, 0, 0" 1.0 1.0 0.0 0 0 0 0)
      (CallFunction|ResetWeapon))))

(event Custom|ResetWeapon
  (Utilities|FlowControl|DoOnce false) ; enters at Reset
)

(event EventBeginPlay)

(event Collision|EventActorBeginOverlap
  (params (OtherActor :type Actor%20Object%20Reference)))

(event EventTick
  (params (DeltaSeconds :type Float%20%28single-precision%29)))

(fn ConstructionScript)

(fn FireWeapon
  (bind _linetrace (Variables|Default|GetLinetrace))
  (bind _returnvalue (Transformation|GetWorldLocation _linetrace))
  (bind (_outhit _returnvalue_2) (Collision|LineTraceForObjects _returnvalue (+ _returnvalue (* (Math|Vector|GetForwardVector (Transformation|GetWorldRotation _linetrace)) (Variables|Default|GetRange))) (Utilities|Array|MakeArray "ObjectTypeQuery1" "ObjectTypeQuery2" "ObjectTypeQuery3") false (Utilities|Array|MakeArray self (Game|GetPlayerCharacter 0)) "ForDuration"))
  (if _returnvalue_2
    (Game|Damage|ApplyDamage (.HitActor (Collision|BreakHitResult _outhit)) (Variables|Default|GetWeaponDamage) 0 0)))