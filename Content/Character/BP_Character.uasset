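; Player character Blueprint handling interaction, pickups, two-slot weapons, grenades and saving.
; A sphere overlap flags the nearby actor by tag, so Interact can trigger it, consume it or swap weapons, dropping the old one.
; The active weapon is a child actor whose class changes on switch, with buffers preserving the other slot's ammo.
; BeginPlay restores position, weapons and grenade counts from SG_gameSave; P saves and L reapplies them.
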(event OnComponentBeginOverlap(Sphere1)
  (params (OverlappedComponent :type Primitive%20Component%20Object%20Reference) (OtherActor :type Actor%20Object%20Reference) (OtherComp :type Primitive%20Component%20Object%20Reference) (OtherBodyIndex :type Integer) (bFromSweep :type Boolean) (SweepResult :type Hit%20Result%20Structure%20%28by%20ref%29))
  ;[1 1 1] INteractibles
  (bind _output_get (Variables|Default|SetOther%20Actor OtherActor))
  (if (Actor|ActorHasTag _output_get "Interact")
    (Variables|Default|SetCanInteract true)
    (elif (Actor|ActorHasTag _output_get "PickUp")
      (Variables|Default|SetCanPickUp true)
      (elif (Actor|ActorHasTag _output_get "Weapon")
        (Variables|Default|SetCanChange true)))))

(event OnComponentEndOverlap(Sphere1)
  (params (OverlappedComponent :type Primitive%20Component%20Object%20Reference) (OtherActor :type Actor%20Object%20Reference) (OtherComp :type Primitive%20Component%20Object%20Reference) (OtherBodyIndex :type Integer))
  ;[1 1 1] INteractibles
  (if (Actor|ActorHasTag OtherActor "Interact")
    (Variables|Default|SetCanInteract false)
    (Variables|Default|SetOther%20Actor 0 :!label _label)
    (elif (Actor|ActorHasTag OtherActor "PickUp")
      (Variables|Default|SetCanPickUp false)
      (goto _label)
      (elif (Actor|ActorHasTag OtherActor "Weapon")
        (Variables|Default|SetCanChange false)
        (goto _label)))))

(event Custom|useAmmo
  (bind _mainweapon (Variables|Default|GetMainWeapon))
  ;[0 0 0] Shoot system
  (Utilities|FlowControl|DoOnce false) ; enters at Reset
)

(event Custom|CanLunchNewNade
  (bind _returnvalue (Game|GetPlayerCameraManager 0))
  ;[0.2133 0.3854 0.07964 0.74] LunchGrenade
  (Utilities|FlowControl|DoOnce false) ; enters at Reset
)

(event Custom|AddGrenade
  (params (Value :type Integer) (GrenadeType :type Integer))
  (bind _grenadenb (Variables|Default|GetGrenadeNb))
  (bind _output (Utilities|Array|Get(acopy) _grenadenb GrenadeType))
  (bind _returnvalue (+ Value _output))
  ;[1 1 1] Collectable
  (if (> _returnvalue 4)
    (Utilities|Array|SetArrayElem (Variables|Default|GetGrenadeNb) GrenadeType 4)
    (else
      (Utilities|Array|SetArrayElem (Variables|Default|GetGrenadeNb) GrenadeType _returnvalue)))
  (Development|PrintString (Utilities|String|Append (Utilities|String|ToString(Integer) (Utilities|Array|Get(acopy) (Variables|Default|GetGrenadeNb) GrenadeType)) " of grenade " (Utilities|String|ToString(Integer) GrenadeType))))

(event Custom|AddHeal
  (params (Value :type Integer))
  ;[1 1 1] Collectable
  (Development|PrintString (Utilities|String|Append (Utilities|String|ToString(Integer) Value) "health") true true "(R=0.269060,G=1.000000,B=0.000000,A=1.000000)"))

(event Custom|AddAmmo
  (params (Value :type Integer) (WeaponName :type Name) (Collectable :type Actor%20Object%20Reference))
  ;[1 1 1] Collectable
  (bind _returnvalue (Actor|GetActorOfClass (Utilities|Array|Get(acopy) (Variables|Default|GetNewWeapon))))
  (if (== WeaponName (Variables|/Game/Blueprint/BaseBP/BP_Weapon.BP_Weapon_C|GetWeaponName _returnvalue))
    (if (>= (Variables|/Game/Blueprint/BaseBP/BP_Weapon.BP_Weapon_C|GetMaxAmmo _returnvalue) (Variables|/Game/Blueprint/BaseBP/BP_Weapon.BP_Weapon_C|GetActualAmmo _returnvalue))
      (Variables|/Game/Blueprint/BaseBP/BP_Weapon.BP_Weapon_C|SetActualAmmo _returnvalue (+ (Variables|/Game/Blueprint/BaseBP/BP_Weapon.BP_Weapon_C|GetActualAmmo _returnvalue) Value))
      (Actor|DestroyActor Collectable)
      (if (>= (Variables|/Game/Blueprint/BaseBP/BP_Weapon.BP_Weapon_C|GetMaxAmmo _returnvalue) (Variables|/Game/Blueprint/BaseBP/BP_Weapon.BP_Weapon_C|GetActualAmmo _returnvalue))
        (Variables|/Game/Blueprint/BaseBP/BP_Weapon.BP_Weapon_C|SetActualAmmo _returnvalue (Variables|/Game/Blueprint/BaseBP/BP_Weapon.BP_Weapon_C|GetMaxAmmo _returnvalue))))))

(event Custom|LoadWeapon
  (bind _newweapon (Variables|Default|GetNewWeapon))
  (bind _childactor (Variables|Default|GetChildActor))
  (bind _output (Utilities|Array|Get(acopy) _newweapon 1))
  (bind _childactor_2 (Variables|/Script/Engine.ChildActorComponent|GetChildActor _childactor))
  (bind (_range _weapondamage _maxammo _actualammo _firesound _actualammoinmagazine _maxammoinmagazine) (Utilities|GetClassDefaults _output))
  ;[0.7587 0.3857 1] Sets your Weapons
  (Variables|Default|SetBufferAAmmo _actualammo)
  (Variables|Default|SetBufferAAmmoIM _actualammoinmagazine)
  (Variables|Default|SetBufferMAmmo _maxammo)
  (Variables|Default|SetBufferMAmmoIM _maxammoinmagazine)
  (ChildActorComponent|SetChildActorClass (Variables|Default|GetChildActor) (Utilities|Array|Get(acopy) (Variables|Default|GetNewWeapon)))
  (bind _asbp_weapon (Utilities|Casting|CastToBP_Weapon _childactor_2))
  (Variables|Default|SetMainWeapon _asbp_weapon)
  (for _array_element (Components|GetChildrenComponents (Variables|/Script/Engine.Actor|GetRootComponent _childactor_2) true)
    (bind _asstatic_mesh_component (Utilities|Casting|CastToStaticMeshComponent _array_element))
    (Collision|SetCollisionEnabled _asstatic_mesh_component "NoCollision")))

(event Input|EnhancedActionEvents|EnhancedInputActionIA_Reload
  (params (ActionValue :type Boolean) (ElapsedSeconds :type Float%20%28double-precision%29) (TriggeredSeconds :type Float%20%28double-precision%29) (InputAction :type Input%20Action%20Object%20Reference :default "/Game/Input/IA_Reload.IA_Reload"))
  (bind _mainweapon (Variables|Default|GetMainWeapon))
  (bind _mainweapon_2 (Variables|Default|GetMainWeapon))
  ;[1 1 1] Reload Weapon
  (:Started
    (if (> (Variables|/Game/Blueprint/BaseBP/BP_Weapon.BP_Weapon_C|GetActualAmmo _mainweapon_2) (- (Variables|/Game/Blueprint/BaseBP/BP_Weapon.BP_Weapon_C|GetMaxAmmoInMagazine _mainweapon_2) (Variables|/Game/Blueprint/BaseBP/BP_Weapon.BP_Weapon_C|GetActualAmmoInMagazine _mainweapon_2)))
      (Variables|/Game/Blueprint/BaseBP/BP_Weapon.BP_Weapon_C|SetActualAmmo _mainweapon (- (Variables|/Game/Blueprint/BaseBP/BP_Weapon.BP_Weapon_C|GetActualAmmo _mainweapon_2) (- (Variables|/Game/Blueprint/BaseBP/BP_Weapon.BP_Weapon_C|GetMaxAmmoInMagazine _mainweapon_2) (Variables|/Game/Blueprint/BaseBP/BP_Weapon.BP_Weapon_C|GetActualAmmoInMagazine _mainweapon_2))))
      (Variables|/Game/Blueprint/BaseBP/BP_Weapon.BP_Weapon_C|SetActualAmmoInMagazine _mainweapon (Variables|/Game/Blueprint/BaseBP/BP_Weapon.BP_Weapon_C|GetMaxAmmoInMagazine _mainweapon))
      (else
        (Development|PrintString "Not enough Ammos")))))

(event Input|EnhancedActionEvents|EnhancedInputActionIA_Nade
  (params (ActionValue :type Boolean) (ElapsedSeconds :type Float%20%28double-precision%29) (TriggeredSeconds :type Float%20%28double-precision%29) (InputAction :type Input%20Action%20Object%20Reference :default "/Game/Input/IA_Nade.IA_Nade"))
  (bind _returnvalue (Game|GetPlayerCameraManager 0))
  ;[0.2133 0.3854 0.07964 0.74] LunchGrenade
  (:Started
    (Utilities|FlowControl|DoOnce false
      (:Completed
        (if (<= (Utilities|Array|Get(acopy) (Variables|Default|GetGrenadeNb) (Variables|Default|GetGrenadeType)) 0)
          (Development|PrintString "No nade")
          (else
            (Game|SpawnActorfromClass (Utilities|Array|Get(acopy) (Variables|Default|GetGrenade_BP_Class) (Variables|Default|GetGrenadeType)) (Math|Transform|MakeTransform (Camera|GetCameraLocation _returnvalue) (Camera|GetCameraRotation _returnvalue)) "Undefined" "MultiplyWithRoot" 0 0)
            (Utilities|Array|SetArrayElem (Variables|Default|GetGrenadeNb) (Variables|Default|GetGrenadeType) (- (Utilities|Array|Get(acopy) (Variables|Default|GetGrenadeNb) (Variables|Default|GetGrenadeType)) 1))
            (Utilities|FlowControl|Delay (Variables|Default|GetGrenadeDelay))))
        (CallFunction|CanLunchNewNade)))))

(event Input|EnhancedActionEvents|EnhancedInputActionIA_ChangeGun
  (params (ActionValue :type Boolean) (ElapsedSeconds :type Float%20%28double-precision%29) (TriggeredSeconds :type Float%20%28double-precision%29) (InputAction :type Input%20Action%20Object%20Reference :default "/Game/Input/IA_ChangeGun.IA_ChangeGun"))
  ;[0.7587 0.3857 1] Change your weapon
  (if ActionValue
    (Variables|Default|SetTmpBuffAAmmo (Variables|Default|GetBufferAAmmo))
    (Variables|Default|SetTmpBuffAAmmoIM (Variables|Default|GetBufferAAmmoIM))
    (Variables|Default|SetTmpBuffMAmmo (Variables|Default|GetBufferMAmmo))
    (Variables|Default|SetTmpBuffMAmmoIM (Variables|Default|GetBufferMAmmoIM))
    (Variables|Default|SetBufferAAmmo (Variables|/Game/Blueprint/BaseBP/BP_Weapon.BP_Weapon_C|GetActualAmmo (Variables|Default|GetMainWeapon)))
    (Variables|Default|SetBufferAAmmoIM (Variables|/Game/Blueprint/BaseBP/BP_Weapon.BP_Weapon_C|GetActualAmmoInMagazine (Variables|Default|GetMainWeapon)))
    (Variables|Default|SetBufferMAmmo (Variables|/Game/Blueprint/BaseBP/BP_Weapon.BP_Weapon_C|GetMaxAmmo (Variables|Default|GetMainWeapon)))
    (Variables|Default|SetBufferMAmmoIM (Variables|/Game/Blueprint/BaseBP/BP_Weapon.BP_Weapon_C|GetMaxAmmoInMagazine (Variables|Default|GetMainWeapon)))
    (if (Variables|Default|GetChangedWeapon?)
      (Variables|Default|SetChangedWeapon? false)
      (else
        (Variables|Default|SetChangedWeapon? true)))
    (ChildActorComponent|SetChildActorClass (Variables|Default|GetChildActor) (Utilities|Array|Get(acopy) (Variables|Default|GetNewWeapon) (Math|Conversions|ToInteger(Boolean) (Variables|Default|GetChangedWeapon?))))
    (bind _asbp_weapon (Utilities|Casting|CastToBP_Weapon (Variables|/Script/Engine.ChildActorComponent|GetChildActor (Variables|Default|GetChildActor))))
    (bind _output_get (Variables|Default|SetMainWeapon _asbp_weapon))
    (Variables|/Game/Blueprint/BaseBP/BP_Weapon.BP_Weapon_C|SetActualAmmo _output_get (Variables|Default|GetTmpBuffAAmmo))
    (Variables|/Game/Blueprint/BaseBP/BP_Weapon.BP_Weapon_C|SetActualAmmoInMagazine _output_get (Variables|Default|GetTmpBuffAAmmoIM))
    (Variables|/Game/Blueprint/BaseBP/BP_Weapon.BP_Weapon_C|SetMaxAmmo _output_get (Variables|Default|GetTmpBuffMAmmo))
    (Variables|/Game/Blueprint/BaseBP/BP_Weapon.BP_Weapon_C|SetMaxAmmoInMagazine _output_get (Variables|Default|GetTmpBuffMAmmoIM))
    (for _array_element (Components|GetChildrenComponents (Variables|/Script/Engine.Actor|GetRootComponent _asbp_weapon) true)
      (bind _asstatic_mesh_component (Utilities|Casting|CastToStaticMeshComponent _array_element))
      (Collision|SetCollisionEnabled _asstatic_mesh_component "NoCollision"))))

(event Input|EnhancedActionEvents|EnhancedInputActionIA_Shoot
  (params (ActionValue :type Boolean) (ElapsedSeconds :type Float%20%28double-precision%29) (TriggeredSeconds :type Float%20%28double-precision%29) (InputAction :type Input%20Action%20Object%20Reference :default "/Game/Input/IA_Shoot.IA_Shoot"))
  (bind _mainweapon (Variables|Default|GetMainWeapon))
  ;[0 0 0] Shoot system
  (Utilities|FlowControl|DoOnce false
    (:Completed
      (if (> (Variables|/Game/Blueprint/BaseBP/BP_Weapon.BP_Weapon_C|GetActualAmmoInMagazine (Variables|Default|GetMainWeapon)) 0)
        (Variables|/Game/Blueprint/BaseBP/BP_Weapon.BP_Weapon_C|SetActualAmmoInMagazine _mainweapon (- (Variables|/Game/Blueprint/BaseBP/BP_Weapon.BP_Weapon_C|GetActualAmmoInMagazine (Variables|Default|GetMainWeapon)) 1))
        (Default|Shoot _mainweapon)
        (Utilities|FlowControl|Delay (Variables|/Game/Blueprint/BaseBP/BP_Weapon.BP_Weapon_C|GetCooldown _mainweapon))
        (CallFunction|UseAmmo)
        (Development|PrintString (Utilities|String|ToString(Integer) (Variables|/Game/Blueprint/BaseBP/BP_Weapon.BP_Weapon_C|GetActualAmmoInMagazine (Variables|Default|GetMainWeapon))))
        (else
          (CallFunction|UseAmmo))))))

(event Input|EnhancedActionEvents|EnhancedInputActionIA_Interact
  (params (ActionValue :type Boolean) (ElapsedSeconds :type Float%20%28double-precision%29) (TriggeredSeconds :type Float%20%28double-precision%29) (InputAction :type Input%20Action%20Object%20Reference :default "/Game/Input/IA_Interact.IA_Interact"))
  (bind _newweapon (Variables|Default|GetNewWeapon))
  (bind _childactor (Variables|Default|GetChildActor))
  (bind _changedweapon_ (Variables|Default|GetChangedWeapon?))
  (bind _returnvalue (Math|Conversions|ToInteger(Boolean) _changedweapon_))
  ;[1 1 1] INteractibles
  (:Started
    (if (Variables|Default|GetCanInteract)
      (bind _asbp_interact (Utilities|Casting|CastToBP_Interact (stale OnComponentBeginOverlap(Sphere1) _output_get))
        (:then
          (Default|SameScaleManage _asbp_interact)
          (if (Variables|Default|GetCanPickUp) :!label _label
            (bind _asbp_pickable (Utilities|Casting|CastToBP_Pickable (stale OnComponentBeginOverlap(Sphere1) _output_get)))
            (Development|PrintString (Utilities|String|ToString(Integer) (Variables|/Game/Blueprint/BaseBP/BP_Pickable.BP_Pickable_C|GetHealValue _asbp_pickable)) true true "(R=1.000000,G=0.000000,B=0.011039,A=1.000000)")
            (Actor|DestroyActor _asbp_pickable)
            (Variables|Default|SetOther%20Actor (stale _returnvalue_2) :!label _label_2)
            (elif (Variables|Default|GetCanChange)
              (Variables|Default|SetBuffClass (Utilities|Array|Get(acopy) _newweapon _returnvalue))
              (bind _asbp_weapon (Utilities|Casting|CastToBP_Weapon (stale OnComponentBeginOverlap(Sphere1) _output_get)))
              (Variables|Default|SetBuffDropTransform (Transformation|GetActorTransform _asbp_weapon))
              (Utilities|Array|SetArrayElem _newweapon _returnvalue (Utilities|GetClass _asbp_weapon))
              (ChildActorComponent|SetChildActorClass _childactor (Utilities|GetClass _asbp_weapon))
              (bind _asbp_weapon_2 (Utilities|Casting|CastToBP_Weapon (Variables|/Script/Engine.ChildActorComponent|GetChildActor _childactor)))
              (bind _output_get (Variables|Default|SetMainWeapon _asbp_weapon_2))
              (for _array_element (Components|GetChildrenComponents (Variables|/Script/Engine.Actor|GetRootComponent _output_get) true)
                (bind _asstatic_mesh_component (Utilities|Casting|CastToStaticMeshComponent _array_element))
                (Collision|SetCollisionEnabled _asstatic_mesh_component "NoCollision"))
              (Actor|DestroyActor _asbp_weapon)
              (bind _returnvalue_2 (Game|SpawnActorfromClass (Variables|Default|GetBuffClass) (Variables|Default|GetBuffDropTransform) "Undefined" "MultiplyWithRoot" 0 0))
              (goto _label_2))))
        (:CastFailed
          (Development|PrintString "blblbblbblb")))
      (else
        (goto _label)))))

(event EventBeginPlay
  (bind _childactor (Variables|Default|GetChildActor))
  (bind _childactor_2 (Variables|/Script/Engine.ChildActorComponent|GetChildActor _childactor))
  ;[0.7587 0.3857 1] Sets your Weapons
  (bind _returnvalue (SaveGame|DoesSaveGameExist "save"))
  (if _returnvalue
    ;[1 1 1] Save System
    (bind _returnvalue_2 (SaveGame|LoadGamefromSlot "save"))
    (bind _assg_game_save (Utilities|Casting|CastToSG_gameSave _returnvalue_2))
    (Variables|Default|SetSave _assg_game_save)
    (Variables|Default|SetNewWeapon (Variables|/Game/Manage/SG_gameSave.SG_gameSave_C|GetNewWeapon _assg_game_save))
    (Variables|Default|SetGrenadeNb (Variables|/Game/Manage/SG_gameSave.SG_gameSave_C|GetGrenadesnb _assg_game_save))
    (Transformation|SetActorTransform (Variables|/Game/Manage/SG_gameSave.SG_gameSave_C|GetPlayerPos _assg_game_save))
    (Variables|Default|SetBufferAAmmo (.ActualAmmo (Utilities|GetClassDefaults (Utilities|Array|Get(acopy) (Variables|Default|GetNewWeapon) 1))) :!label _label)
    (Variables|Default|SetBufferAAmmoIM (.ActualAmmoInMagazine (Utilities|GetClassDefaults (Utilities|Array|Get(acopy) (Variables|Default|GetNewWeapon) 1))))
    (Variables|Default|SetBufferMAmmo (.MaxAmmo (Utilities|GetClassDefaults (Utilities|Array|Get(acopy) (Variables|Default|GetNewWeapon) 1))))
    (Variables|Default|SetBufferMAmmoIM (.MaxAmmoInMagazine (Utilities|GetClassDefaults (Utilities|Array|Get(acopy) (Variables|Default|GetNewWeapon) 1))))
    (ChildActorComponent|SetChildActorClass (Variables|Default|GetChildActor) (Utilities|Array|Get(acopy) (Variables|Default|GetNewWeapon)))
    (bind _asbp_weapon (Utilities|Casting|CastToBP_Weapon _childactor_2))
    (Variables|Default|SetMainWeapon _asbp_weapon)
    (for _array_element (Components|GetChildrenComponents (Variables|/Script/Engine.Actor|GetRootComponent _childactor_2) true)
      (bind _asstatic_mesh_component (Utilities|Casting|CastToStaticMeshComponent _array_element))
      (Collision|SetCollisionEnabled _asstatic_mesh_component "NoCollision"))
    (else
      (Utilities|FlowControl|Sequence
        (:then_0
          (goto _label))
        (:then_1
          (bind _returnvalue_3 (SaveGame|CreateSaveGameObject "/Game/Manage/SG_gameSave.SG_gameSave_C"))
          (bind _output_get (Variables|Default|SetSave _returnvalue_3))
          (Variables|/Game/Manage/SG_gameSave.SG_gameSave_C|SetPlayerPos _output_get (Transformation|GetActorTransform))
          (Variables|/Game/Manage/SG_gameSave.SG_gameSave_C|SetNewWeapon _output_get (Variables|Default|GetNewWeapon))
          (Variables|/Game/Manage/SG_gameSave.SG_gameSave_C|SetGrenadesnb _output_get (Variables|Default|GetGrenadeNb))
          (SaveGame|SaveGametoSlot _output_get "save"))))))

(event Input|KeyboardEvents|P
  (params (Key :type Key%20Structure :default "None"))
  (bind _save (Variables|Default|GetSave))
  (:Pressed
    (Variables|/Game/Manage/SG_gameSave.SG_gameSave_C|SetPlayerPos _save (Transformation|GetActorTransform))
    (Variables|/Game/Manage/SG_gameSave.SG_gameSave_C|SetNewWeapon _save (Variables|Default|GetNewWeapon))
    (Variables|/Game/Manage/SG_gameSave.SG_gameSave_C|SetGrenadesnb _save (Variables|Default|GetGrenadeNb))
    (SaveGame|SaveGametoSlot _save "save")))

(event Input|KeyboardEvents|L
  (params (Key :type Key%20Structure :default "None"))
  (bind _save (Variables|Default|GetSave))
  (:Pressed
    (Variables|Default|SetNewWeapon (Variables|/Game/Manage/SG_gameSave.SG_gameSave_C|GetNewWeapon _save))
    (Variables|Default|SetGrenadeNb (Variables|/Game/Manage/SG_gameSave.SG_gameSave_C|GetGrenadesnb _save))
    (Transformation|SetActorTransform (Variables|/Game/Manage/SG_gameSave.SG_gameSave_C|GetPlayerPos _save))
    (CallFunction|LoadWeapon)))

(fn ConstructionScript)