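; Actor component that gives the player character a hold-to-grapple ability with a visible cable.
; A setup event caches the owner's camera and the supplied cable, then shooting line-traces forward from the camera to set the grab point.
; On a hit it switches movement to Flying, and Tick pins the cable end to that point while applying force toward it.
; Releasing the input hides the cable and returns movement to Falling.
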(event Custom|BreackLoop
  ;[1 0 0.1309] Show camera reférence
  (Utilities|Array|ForEachLoopwithBreak (Components|GetChildrenComponents (Variables|/Script/Engine.Actor|GetRootComponent (Components|GetOwner)) true)) ; enters at Break
)

(event Custom|CustomEvent
  (params (YourCabble :type Cable%20Component%20Object%20Reference))
  ;[1 0 0.1309] Show camera reférence
  (bind _array_element (Utilities|Array|ForEachLoopwithBreak (Components|GetChildrenComponents (Variables|/Script/Engine.Actor|GetRootComponent (Components|GetOwner)) true))
    (:LoopBody
      (if (== _array_element "/Script/Engine.CameraComponent")
        (Variables|Default|SetCamRef _array_element)
        (Variables|Default|SetCable YourCabble)
        (CallFunction|BreackLoop)))))

(event Input|EnhancedActionEvents|EnhancedInputActionIA_Shoot
  (params (ActionValue :type Boolean) (ElapsedSeconds :type Float%20%28double-precision%29) (TriggeredSeconds :type Float%20%28double-precision%29) (InputAction :type Input%20Action%20Object%20Reference :default "/Game/Input/IA_Shoot.IA_Shoot"))
  (bind _camref (Variables|Default|GetCamRef))
  (bind _cable (Variables|Default|GetCable))
  (bind _returnvalue (Transformation|GetWorldLocation _camref))
  ;[0 0.4 0.4] Grappling System
  (:Started
    (Development|PrintString "Shoot")
    (bind (_outhit _returnvalue_2) (Collision|LineTraceByChannel _returnvalue (+ _returnvalue (* (Math|Vector|GetForwardVector (Transformation|GetWorldRotation _camref)) (Variables|Default|GetRange))) "TraceTypeQuery1" false 0 "ForDuration"))
    (if _returnvalue_2
      (Variables|Default|SetGrabPoint (.ImpactPoint (Collision|BreakHitResult _outhit)))
      (Variables|Default|SetIsGrappling true)
      (Pawn|Components|CharacterMovement|SetMovementMode (Variables|/Script/Engine.Character|GetCharacterMovement (Game|GetPlayerCharacter 0)) "MOVE_Flying" 0)
      (Utilities|IsValid _cable
        (:Is%20Valid
          (Rendering|SetVisibility _cable true false)
          (Audio|PlaySoundatLocation (Variables|Default|GetSoundShoot) (Transformation|GetWorldLocation (Variables|Default|GetCable)) "0, 0, 0" 1.0 1.0 0.0 0 0 0 0) ; Play firing sound
        ))))
  (:Completed
    (Variables|Default|SetIsGrappling false)
    (Pawn|Components|CharacterMovement|SetMovementMode (Variables|/Script/Engine.Character|GetCharacterMovement (Game|GetPlayerCharacter 0)) "MOVE_Falling" 0)
    (Rendering|SetVisibility (Variables|Default|GetCable) false false)))

(event EventTick
  (params (DeltaSeconds :type Float%20%28single-precision%29))
  (bind _returnvalue (Game|GetPlayerCharacter 0))
  ;[0 0.4 0.4] Graplling aspect and force
  (Utilities|IsValid (Variables|Default|GetCable)
    (:Is%20Valid
      (if (Variables|Default|GetIsGrappling)
        (Variables|/Script/CableComponent.CableComponent|SetEndLocation (Variables|Default|GetCable) (Math|Transform|InverseTransformLocation (Transformation|GetActorTransform _returnvalue) (Variables|Default|GetGrabPoint)))
        (Physics|AddForce (Variables|/Script/Engine.Character|GetCharacterMovement (Game|GetPlayerCharacter 0)) (* (Math|Vector|Normalize (+ (Math|Vector|GetUnitDirection(Vector) (Transformation|GetActorLocation _returnvalue) (Variables|Default|GetGrabPoint)) (* (Transformation|GetActorRightVector _returnvalue) ""))) (* (Variables|Default|GetForce) 1e+04)))))))